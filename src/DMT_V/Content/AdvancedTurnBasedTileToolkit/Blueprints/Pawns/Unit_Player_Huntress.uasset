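; Huntress player unit for the turn-based tile toolkit, extending its parent unit's events with calls into the character's animation Blueprint.
; Attack and destroy trigger attack and death animations, while damage plays a hit reaction after a delay if health remains.
; Tick calls the move animation once on becoming idle and every frame otherwise, also clearing the break flag.
; A self-rearming random timer plays break animations periodically.
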(event Custom|RandomizeBreakTimer
  (Utilities|Time|SetTimerbyFunctionName 0 "BreakTimer" (Math|Random|RandomFloatinRange 1e+01 2e+01)))

(event EventTick
  (params (DeltaSeconds :type Float%20%28single-precision%29))
  (bind _skeletalmesh (Variables|Default|GetSkeletalMesh))
  (bind _returnvalue (Components|SkeletalMesh|GetAnimInstance _skeletalmesh))
  (bind _ashuntress_anim_bp_parent (Utilities|Casting|CastToHuntress_Anim_BP_Parent _returnvalue))
  (|CallParentFunction DeltaSeconds)
  (if (Variables|Default|GetIdle)
    (Utilities|FlowControl|DoOnce true :!label _label
      (:Completed
        _))
    (else
      (Utilities|FlowControl|Sequence
        (:then_0
          (goto _label Reset))
        (:then_1
          (Variables|/Game/AdvancedTurnBasedTileToolkit/Animations/Huntress/Huntress_Anim_BP_Parent.Huntress_Anim_BP_Parent_C|SetBreak _ashuntress_anim_bp_parent false)))))
  (Default|MoveAnimation _ashuntress_anim_bp_parent))

(event EventAttackVictim
  (params (Victim :type Unit%20Parent%20Object%20Reference))
  (|CallParentFunction Victim)
  (bind _ashuntress_anim_bp_parent (Utilities|Casting|CastToHuntress_Anim_BP_Parent (Components|SkeletalMesh|GetAnimInstance (Variables|Default|GetSkeletalMesh))))
  (Default|AttackAnimation _ashuntress_anim_bp_parent))

(event EventDestroyUnit
  (params (Anim%20Delay :type Float%20%28single-precision%29))
  (|CallParentFunction Anim%20Delay)
  (bind _ashuntress_anim_bp_parent (Utilities|Casting|CastToHuntress_Anim_BP_Parent (Components|SkeletalMesh|GetAnimInstance (Variables|Default|GetSkeletalMesh))))
  (Default|DeathAnimation _ashuntress_anim_bp_parent))

(event EventBeginPlay
  (|CallParentFunction)
  (Utilities|Time|SetTimerbyFunctionName 0 "BreakTimer" (Math|Random|RandomFloatinRange 1e+01 2e+01)))

(event EventDamage
  (params (Damage :type Float%20%28single-precision%29) (Anim%20Delay :type Float%20%28single-precision%29))
  (|CallParentFunction Damage Anim%20Delay)
  (Utilities|FlowControl|Delay Anim%20Delay)
  (if (> (Variables|Default|GetCurrentHealth) 0.0)
    (bind _ashuntress_anim_bp_parent (Utilities|Casting|CastToHuntress_Anim_BP_Parent (Components|SkeletalMesh|GetAnimInstance (Variables|Default|GetSkeletalMesh))))
    (Default|HitAnimation _ashuntress_anim_bp_parent)))

(fn ConstructionScript
  (|CallParentFunction))

(fn BreakTimer
  (bind _aspawn_anim_bp_parent (Utilities|Casting|CastToPawn_Anim_BP_Parent (Components|SkeletalMesh|GetAnimInstance (Variables|Default|GetSkeletalMesh))))
  (Default|BreakAnimation _aspawn_anim_bp_parent)
  (CallFunction|RandomizeBreakTimer))