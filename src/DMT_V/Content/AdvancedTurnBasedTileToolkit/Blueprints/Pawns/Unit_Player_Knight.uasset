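; Player knight unit pawn for the turn-based tile toolkit, extending its parent unit with skeletal mesh animation.
; Each override calls the parent, then drives Knight_Anim_BP_Parent through a cast of the mesh's anim instance.
; Attack and destroy events trigger attack and death animations.
; Tick clears Break and calls MoveAnimation every frame while not Idle, with a DoOnce limiting it to one call on becoming Idle.
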(event EventTick
  (params (DeltaSeconds :type Float%20%28single-precision%29))
  (bind _skeletalmesh (Variables|Default|GetSkeletalMesh))
  (bind _returnvalue (Components|SkeletalMesh|GetAnimInstance _skeletalmesh))
  (bind _asknight_anim_bp_parent (Utilities|Casting|CastToKnight_Anim_BP_Parent _returnvalue))
  (|CallParentFunction DeltaSeconds)
  (if (Variables|Default|GetIdle)
    (Utilities|FlowControl|DoOnce true :!label _label
      (:Completed
        _))
    (else
      (Utilities|FlowControl|Sequence
        (:then_0
          (goto _label Reset))
        (:then_1
          (Variables|/Game/AdvancedTurnBasedTileToolkit/Animations/Knight/Knight_Anim_BP_Parent.Knight_Anim_BP_Parent_C|SetBreak _asknight_anim_bp_parent false)))))
  (Default|MoveAnimation _asknight_anim_bp_parent))

(event EventAttackVictim
  (params (Victim :type Unit%20Parent%20Object%20Reference))
  (|CallParentFunction Victim)
  (bind _asknight_anim_bp_parent (Utilities|Casting|CastToKnight_Anim_BP_Parent (Components|SkeletalMesh|GetAnimInstance (Variables|Default|GetSkeletalMesh))))
  (Default|AttackAnimation _asknight_anim_bp_parent))

(event EventDestroyUnit
  (params (Anim%20Delay :type Float%20%28single-precision%29))
  (|CallParentFunction Anim%20Delay)
  (bind _asknight_anim_bp_parent (Utilities|Casting|CastToKnight_Anim_BP_Parent (Components|SkeletalMesh|GetAnimInstance (Variables|Default|GetSkeletalMesh))))
  (Default|DeathAnimation _asknight_anim_bp_parent))

(event EventBeginPlay
  (|CallParentFunction))

(fn ConstructionScript
  (|CallParentFunction))