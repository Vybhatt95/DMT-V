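; Player-controlled Mage unit pawn for a turn-based tile game, extending a parent unit with mage animations and starting gear.
; Move, attack, damage and death events call the parent, then trigger matching animations on the mage Anim Blueprint.
; A random timer plays idle break animations, then re-enters the BeginPlay setup chain, which also hides the health billboard, sets the class and adds staff, kilt and potions again.
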(event Custom|RandomizeBreakTimer
  (bind _playerinventory (Variables|Default|GetPlayerInventory))
  (Utilities|Time|SetTimerbyFunctionName 0 "BreakTimer" (Math|Random|RandomFloatinRange 1e+01 2e+01))
  (Rendering|SetVisibility (Variables|Default|GetHealthBillboard) false false)
  (Variables|Default|SetClass "NewEnumerator1")
  (Utilities|Array|Add _playerinventory (Utilities|Struct|MakeStruct_Item "Oak Staff" "/Game/AdvancedTurnBasedTileToolkit/Textures/ItemThumbnails/Mage/staff00.staff00" true "NewEnumerator1" 30 false "NewEnumerator5" 0 "NewEnumerator1" false false (Math|Random|RandomInteger 10000) 29 0 false))
  (Utilities|Array|Add _playerinventory (Utilities|Struct|MakeStruct_Item "Cloth Kilt" "/Game/AdvancedTurnBasedTileToolkit/Textures/ItemThumbnails/Mage/ClothPants.ClothPants" false "NewEnumerator5" 0 true "NewEnumerator6" 7 "NewEnumerator1" false false (Math|Random|RandomInteger 10000) 10))
  (Utilities|Array|Add _playerinventory (Utilities|Struct|MakeStruct_Item "Health Potion" "/Game/AdvancedTurnBasedTileToolkit/Textures/ItemThumbnails/hp1.hp1" false "NewEnumerator5" 0 false "NewEnumerator5" 0 "NewEnumerator3" true false (Math|Random|RandomIntegerinRange 0 10000) 32))
  (Utilities|Array|Add _playerinventory (Utilities|Struct|MakeStruct_Item "Health Potion" "/Game/AdvancedTurnBasedTileToolkit/Textures/ItemThumbnails/hp1.hp1" false "NewEnumerator5" 0 false "NewEnumerator5" 0 "NewEnumerator3" true false (Math|Random|RandomIntegerinRange 0 10000) 32)))

(event Custom|ReceiveDamage1
  (params (Damage :type Float%20%28single-precision%29) (Anim%20Delay :type Float%20%28single-precision%29))
  (Utilities|FlowControl|Delay Anim%20Delay)
  (if (> (Variables|Default|GetCurrentHealth) 0.0)
    (bind _asmage_anim_bp_parent (Utilities|Casting|CastToMage_Anim_BP_Parent (Components|SkeletalMesh|GetAnimInstance (Variables|Default|GetSkeletalMesh))))
    (Default|HitAnimation _asmage_anim_bp_parent)))

(event EventMoveTimelineUpdateFunc
  (bind _skeletalmesh (Variables|Default|GetSkeletalMesh))
  (bind _returnvalue (Components|SkeletalMesh|GetAnimInstance _skeletalmesh))
  (bind _asmage_anim_bp_parent (Utilities|Casting|CastToMage_Anim_BP_Parent _returnvalue))
  (|CallParentFunction)
  (if (Variables|Default|GetIdle)
    (Utilities|FlowControl|DoOnce true :!label _label
      (:Completed
        _))
    (else
      (Utilities|FlowControl|Sequence
        (:then_0
          (goto _label Reset))
        (:then_1
          (Variables|/Game/AdvancedTurnBasedTileToolkit/Animations/Mage/Mage_Anim_BP_Parent.Mage_Anim_BP_Parent_C|SetBreak _asmage_anim_bp_parent false)))))
  (Default|MoveAnimation _asmage_anim_bp_parent))

(event EventDamage
  (params (Damage :type Float%20%28single-precision%29) (Anim%20Delay :type Float%20%28single-precision%29))
  (|CallParentFunction Damage Anim%20Delay)
  (Utilities|FlowControl|Delay (stale Custom|ReceiveDamage1 Anim%20Delay))
  (if (> (Variables|Default|GetCurrentHealth) 0.0)
    (bind _asmage_anim_bp_parent (Utilities|Casting|CastToMage_Anim_BP_Parent (Components|SkeletalMesh|GetAnimInstance (Variables|Default|GetSkeletalMesh))))
    (Default|HitAnimation _asmage_anim_bp_parent)))

(event EventAttackVictim
  (params (Victim :type Unit%20Object%20Reference))
  (|CallParentFunction Victim)
  (bind _asmage_anim_bp_parent (Utilities|Casting|CastToMage_Anim_BP_Parent (Components|SkeletalMesh|GetAnimInstance (Variables|Default|GetSkeletalMesh))))
  (Default|AttackAnimation _asmage_anim_bp_parent))

(event EventKillUnit
  (params (Anim%20Delay :type Float%20%28single-precision%29))
  (|CallParentFunction Anim%20Delay)
  (bind _asmage_anim_bp_parent (Utilities|Casting|CastToMage_Anim_BP_Parent (Components|SkeletalMesh|GetAnimInstance (Variables|Default|GetSkeletalMesh))))
  (Default|DeathAnimation _asmage_anim_bp_parent))

(event EventBeginPlay
  (bind _playerinventory (Variables|Default|GetPlayerInventory))
  (|CallParentFunction)
  (Utilities|Time|SetTimerbyFunctionName 0 "BreakTimer" (Math|Random|RandomFloatinRange 1e+01 2e+01))
  (Rendering|SetVisibility (Variables|Default|GetHealthBillboard) false false)
  (Variables|Default|SetClass "NewEnumerator1")
  (Utilities|Array|Add _playerinventory (Utilities|Struct|MakeStruct_Item "Oak Staff" "/Game/AdvancedTurnBasedTileToolkit/Textures/ItemThumbnails/Mage/staff00.staff00" true "NewEnumerator1" 30 false "NewEnumerator5" 0 "NewEnumerator1" false false (Math|Random|RandomInteger 10000) 29 0 false))
  (Utilities|Array|Add _playerinventory (Utilities|Struct|MakeStruct_Item "Cloth Kilt" "/Game/AdvancedTurnBasedTileToolkit/Textures/ItemThumbnails/Mage/ClothPants.ClothPants" false "NewEnumerator5" 0 true "NewEnumerator6" 7 "NewEnumerator1" false false (Math|Random|RandomInteger 10000) 10))
  (Utilities|Array|Add _playerinventory (Utilities|Struct|MakeStruct_Item "Health Potion" "/Game/AdvancedTurnBasedTileToolkit/Textures/ItemThumbnails/hp1.hp1" false "NewEnumerator5" 0 false "NewEnumerator5" 0 "NewEnumerator3" true false (Math|Random|RandomIntegerinRange 0 10000) 32))
  (Utilities|Array|Add _playerinventory (Utilities|Struct|MakeStruct_Item "Health Potion" "/Game/AdvancedTurnBasedTileToolkit/Textures/ItemThumbnails/hp1.hp1" false "NewEnumerator5" 0 false "NewEnumerator5" 0 "NewEnumerator3" true false (Math|Random|RandomIntegerinRange 0 10000) 32)))

(fn ConstructionScript
  (|CallParentFunction))

(fn BreakTimer
  (bind _aspawn_anim_bp_parent (Utilities|Casting|CastToPawn_Anim_BP_Parent (Components|SkeletalMesh|GetAnimInstance (Variables|Default|GetSkeletalMesh))))
  (Default|BreakAnimation _aspawn_anim_bp_parent)
  (CallFunction|RandomizeBreakTimer))